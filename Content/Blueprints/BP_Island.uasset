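; BP_Island is an island actor that displays a floating text label that always faces the player's camera.
; On BeginPlay it sets the TextRender to the actor's first tag and caches the camera from the player's BP_TopDownCharacter.
; Every Tick it rotates the label with a look-at rotation toward that camera, producing a billboard effect.
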(event EventBeginPlay
  (Rendering|Components|TextRender|SetText (Variables|Default|GetTextRender) (Utilities|Text|ToText(Name) (Utilities|Array|Get(acopy) (Variables|Actor|GetTags))))
  (bind _asbp_top_down_character (Utilities|Casting|CastToBP_TopDownCharacter (Game|GetPlayerCharacter 0)))
  (Variables|Default|SetCamera (Variables|/Game/TopDown/Blueprints/Charachter/BP_TopDownCharacter.BP_TopDownCharacter_C|GetCamera _asbp_top_down_character)))

(event Collision|EventActorBeginOverlap
  (params (OtherActor :type Actor%20Object%20Reference)))

(event EventTick
  (params (DeltaSeconds :type Float%20%28single-precision%29))
  (Transformation|SetWorldRotation (Variables|Default|GetTextRender) (Math|Rotator|FindLookatRotation (Transformation|GetWorldLocation (Variables|Default|GetTextRender)) (Transformation|GetWorldLocation (Variables|Default|GetCamera))) false false))

(fn ConstructionScript)